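; Player controller Blueprint that switches the game's UI between in-game, inventory and pause states from input actions.
; The inventory input returns to InGame if the inventory is showing, otherwise it calls SwitchToInventory; the pause input sets the Pause state.
; SwitchToInventory passes the in-game widget's MonsterArrayID to the game instance before changing state, and prints a debug string if that widget is not current.
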(event EventBeginPlay)

(event EventTick
  (params (DeltaSeconds :type Float%20%28single-precision%29)))

(event Input|ActionEvents|InputActionInventorySwitch
  (params (Key :type Key%20Structure :default "None"))
  (:Pressed
    (bind _returnvalue (Class|MyPlayerController|GetUIState))
    (bind _returnvalue_2 (Class|MyPlayerController|GetUIStateCheck "UI_Inventory"))
    (if (== _returnvalue _returnvalue_2)
      (Class|MyPlayerController|ChangeUIState "UI_InGame")
      (else
        (CallFunction|SwitchtoInventory)))))

(event Input|ActionEvents|InputActionPauseSwitch
  (params (Key :type Key%20Structure :default "None"))
  (:Pressed
    (Class|MyPlayerController|ChangeUIState "UI_Pause")))

(fn ConstructionScript)

(fn SwitchtoInventory
  (bind _asmy_game_instance (Utilities|Casting|CastToMyGameInstance (Game|GetGameInstance)))
  (bind _aswbp_in_game (Utilities|Casting|CastToWBP_InGame (Variables|Default|GetCurrentWidget))
    (:then
      (Class|MyGameInstance|OnGameWidgetQuit _asmy_game_instance (Variables|/Script/WidgetPraktyki.InGameWidget|GetMonsterArrayID _aswbp_in_game))
      (bind _asmy_player_controller (Utilities|Casting|CastToMyPlayerController (Game|GetPlayerController 0)))
      (Class|MyPlayerController|ChangeUIState _asmy_player_controller "UI_Inventory"))
    (:CastFailed
      (Development|PrintString "Hello"))))